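; BP_Door is a clickable door actor that acts as a voting choice, labelled with a category sign.
; Clicking DoorMesh casts the result of GetGameMode to BP_GameState and calls CastVote with this door's DoorIndex, printing debug messages on press and cast failure.
; SetDoorCategory passes a category name to the WBP_DoorSign widget held by SignWidget to set its text.
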(event `self.DoorMesh.OnClicked`
  (params (TouchedComponent :type "PrimitiveComponent Object Reference") (ButtonPressed :type "Key Structure"))
  (`KismetSystemLibrary.PrintString` "Pressed")
  (bind _asbp_game_state (cast `/Game/_Game/BP_GameState` (`GameplayStatics.GetGameMode`))
    (:`then`
      (`/Game/_Game/BP_GameState.CastVote` _asbp_game_state (`self.DoorIndex`)))
    (:`CastFailed`
      (`KismetSystemLibrary.PrintString` "Failed"))))

(event `SetDoorCategory`
  (params (CategoryName :type String))
  (bind _aswbp_door_sign (cast `/Game/_Game/UI/WBP_DoorSign` (`WidgetComponent.GetUserWidgetObject` (`self.SignWidget`))))
  (`/Game/_Game/UI/WBP_DoorSign.SetCategoryText` _aswbp_door_sign CategoryName))

(fn `UserConstructionScript`)