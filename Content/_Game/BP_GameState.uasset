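; Game state that runs category voting on doors, drawing the categories from a question bank data table.
; On BeginPlay it collects unique main categories, shuffles them, assigns the first four to doors found by indexed "Door" tags, and enables mouse cursor and click events.
; CastVote increments the category's vote count and adds a badge to the matching door's sign widget.
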(event `CastVote`
  (params (CategoryIndex :type Integer))
  (bind _votecounts (`self.VoteCounts`))
  (`KismetArrayLibrary.Array_Set` _votecounts CategoryIndex (+ (`|GetArrayItem` _votecounts CategoryIndex) 1))
  (bind _outactors (`GameplayStatics.GetAllActorsWithTag` (`KismetStringLibrary.Conv_StringToName` (`KismetStringLibrary.Concat_StrStr` "Door" (`KismetStringLibrary.Conv_IntToString` CategoryIndex)))))
  (bind _aswbp_door_sign (cast `/Game/_Game/UI/WBP_DoorSign` (`WidgetComponent.GetUserWidgetObject` (`self.GetComponentByClass` (`|GetArrayItem` _outactors) "/Script/UMG.WidgetComponent"))))
  (`/Game/_Game/UI/WBP_DoorSign.AddVoteBadge` _aswbp_door_sign "/Engine/MapTemplates/TestCard.TestCard"))

(event `self.ReceiveBeginPlay`
  (bind _outrownames (`DataTableFunctionLibrary.GetDataTableRowNames` "/Game/_Game/DT_QuestionBank.DT_QuestionBank"))
  (for _array_element _outrownames
    (bind _returnvalue (`|GetDataTableRow` "/Game/_Game/DT_QuestionBank.DT_QuestionBank" _array_element)
      (:`then`
        (`KismetArrayLibrary.Array_AddUnique` (`self.AvailableMainCategories`) (`KismetStringLibrary.Conv_NameToString` (break `/Game/_Game/S_Quiz` _returnvalue))))))
  (`KismetArrayLibrary.Array_Shuffle` (`self.AvailableMainCategories`))
  (for _index (range 4)
    (bind _outactors (`GameplayStatics.GetAllActorsWithTag` (`KismetStringLibrary.Conv_StringToName` (`KismetStringLibrary.Concat_StrStr` "Door" (`KismetStringLibrary.Conv_IntToString` _index)))))
    (bind _asbp_door (cast `/Game/_Game/BP_Door` (`|GetArrayItem` _outactors)))
    (`/Game/_Game/BP_Door.SetDoorCategory` _asbp_door (`|GetArrayItem` (`self.AvailableMainCategories`) _index)))
  (set `PlayerController.bShowMouseCursor` true (`GameplayStatics.GetPlayerController` 0))
  (set `PlayerController.bEnableClickEvents` true (`GameplayStatics.GetPlayerController` 0))
  (`KismetSystemLibrary.PrintString` "Clicks Enabled!"))

(fn `UserConstructionScript`)