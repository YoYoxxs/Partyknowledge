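; Game state that runs the quiz match loop: intro banner, category door voting, question showcase, timed answering, reveal.
; Votes pick a DT_QuestionBank category whose questions fill tagged answer platforms; wrong platforms are eliminated before a timeline zooms onto the winner.
; Timers and delays chain phases, blending player 0's view between tagged cameras.
; Match events are shuffled at start, but every third question only prints a notice and restarts voting.
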(event `self.ReceiveBeginPlay`
  (`self.SetupMatchEvents`)
  (`self.StartNextQuestion`))

(event `ResetAllPlayerTokens`
  (bind _outactors (`GameplayStatics.GetAllActorsOfClass` "/Game/_Game/BlueprintsCore/BP_PlayerToken.BP_PlayerToken_C"))
  (for _array_element _outactors
    (`/Game/_Game/BlueprintsCore/BP_PlayerToken.ResetPlayerToken` _array_element)
    (`/Game/_Game/BlueprintsCore/BP_PlayerToken.EliminatePlayer` _array_element)))

(event `OnQuestionEnded`
  ;[0.8796 0.8796 0.8796 0.502] GAME LOOP & PROGRESSION
  (`KismetSystemLibrary.K2_ClearAndInvalidateTimerHandle` (`self.TimerHandle`))
  (`Widget.RemoveFromParent` (`self.TimerWidget`))
  (`self.ResetAllDoors`)
  (if (== (mod (`self.CurrentQuestionNumber`) 3) 0)
    (`KismetSystemLibrary.PrintString` "EVENT TIME! Triggering event...")
    (`self.StartDoorVoting`)
    (else
      (set `self.CurrentQuestionNumber` (+ (`self.CurrentQuestionNumber`) 1))
      (`self.StartNextQuestion`))))

(event `SetupDoorCategories`
  ;[0.8796 0.8796 0.8796 0.502] DOOR VOTING PHASE
  (bind _outrownames (`DataTableFunctionLibrary.GetDataTableRowNames` "/Game/_Game/Data/DT_QuestionBank.DT_QuestionBank"))
  (for _array_element _outrownames
    (bind _returnvalue (`|GetDataTableRow` "/Game/_Game/Data/DT_QuestionBank.DT_QuestionBank" _array_element)
      (:`then`
        (`KismetArrayLibrary.Array_AddUnique` (`self.AvailableMainCategories`) (`KismetStringLibrary.Conv_NameToString` (break `/Game/_Game/Data/S_Quiz` _returnvalue))))))
  (`KismetArrayLibrary.Array_Shuffle` (`self.AvailableMainCategories`))
  (for _index (range 4)
    (bind _outactors (`GameplayStatics.GetAllActorsWithTag` (`KismetStringLibrary.Conv_StringToName` (`KismetStringLibrary.Concat_StrStr` "Door" (`KismetStringLibrary.Conv_IntToString` _index)))))
    (bind _asbp_door (cast `/Game/_Game/BlueprintsGameplay/BP_Door` (`|GetArrayItem` _outactors)))
    (`/Game/_Game/BlueprintsGameplay/BP_Door.SetDoorCategory` _asbp_door (`|GetArrayItem` (`self.AvailableMainCategories`) _index)))
  (set `PlayerController.bShowMouseCursor` true (`GameplayStatics.GetPlayerController` 0))
  (set `PlayerController.bEnableClickEvents` true (`GameplayStatics.GetPlayerController` 0))
  (`KismetSystemLibrary.PrintString` "Clicks Enabled!")
  (`KismetSystemLibrary.K2_SetTimerDelegate` (delegate `OnVotingTimeExpired`) 10.0))

(event `StartNextQuestion`
  ;[0.8796 0.8796 0.8796 0.502] QUESTION & ANSWERING PHASE
  (bind _returnvalue (`|CreateWidget` "/Game/_Game/UI/WBP_QuestionIntro.WBP_QuestionIntro_C"))
  (`/Game/_Game/UI/WBP_QuestionIntro.fn_SetBannerText` _returnvalue (`self.CurrentQuestionNumber`) "Knowledge Party")
  (`UserWidget.AddToViewport` _returnvalue 0)
  (`KismetSystemLibrary.Delay` 4.0)
  (`Widget.RemoveFromParent` _returnvalue)
  (`self.StartDoorVoting`))

(event `SetupMatchEvents`
  (bind _activeeventslist (`self.ActiveEventsList`))
  ;[0.8796 0.8796 0.8796 0.502] Comment
  (`KismetArrayLibrary.Array_Shuffle` (`self.AvailableEvents`))
  (`KismetArrayLibrary.Array_Clear` _activeeventslist)
  (`KismetArrayLibrary.Array_Add` _activeeventslist (`|GetArrayItem` (`self.AvailableEvents`)))
  (`KismetArrayLibrary.Array_Add` _activeeventslist (`|GetArrayItem` (`self.AvailableEvents`) 1))
  (`KismetArrayLibrary.Array_Add` _activeeventslist "NewEnumerator3"))

(event `StartQuestionPhase`
  ;[0.8796 0.8796 0.8796 0.502] QUESTION & ANSWERING PHASE
  (bind _output_get (set `self.Current Question Row Name` (`|GetArrayItem` (`self.MatchingRowNames`) (`self.CurrentQuestionNumber`))))
  (bind _returnvalue (`|GetDataTableRow` "/Game/_Game/Data/DT_QuestionBank.DT_QuestionBank" _output_get)
    (:`then`
      (bind _outactors (`GameplayStatics.GetAllActorsWithTag` "QuestionCamera"))
      (`PlayerController.SetViewTargetWithBlend` (`GameplayStatics.GetPlayerController` 0) (`|GetArrayItem` _outactors) 1.5 "VTBlend_EaseInOut" 0.0 false)
      (bind _returnvalue_2 (`|CreateWidget` "/Game/_Game/UI/WBP_QuestionShowcase.WBP_QuestionShowcase_C" null (`.QuestionText_2_3D36EEE940F58E65A419A48BB2DB8745` (break `/Game/_Game/Data/S_Quiz` _returnvalue))))
      (`UserWidget.AddToViewport` _returnvalue_2 0)
      (`KismetSystemLibrary.Delay` 5.0)
      (`Widget.RemoveFromParent` _returnvalue_2)
      (`self.StartAnsweringPhase`))))

(event `OnVotingTimeFinished`)

(event `StartAnsweringPhase`
  (bind _returnvalue (`GameplayStatics.GetPlayerController` 0))
  (bind _timerwidget (`self.TimerWidget`))
  ;[0.8796 0.8796 0.8796 0.502] QUESTION & ANSWERING PHASE
  (bind _outactors (`GameplayStatics.GetAllActorsWithTag` "AnswerCamera"))
  (`self.SetupAnswerPlatforms`)
  (`PlayerController.SetViewTargetWithBlend` (`GameplayStatics.GetPlayerController` 0) (`|GetArrayItem` _outactors) 1.0 "VTBlend_EaseInOut" 0.0 false)
  (set `self.bCanSelectAnswer` true)
  (set `PlayerController.bShowMouseCursor` true _returnvalue)
  (set `PlayerController.bEnableClickEvents` true _returnvalue)
  (`/Engine/EditorBlueprintResources/StandardMacros.IsValid` _timerwidget
    (:`Is Valid`
      (`Widget.RemoveFromParent` _timerwidget))
    (:`Is Not Valid`
      _))
  (bind _returnvalue_2 (`|CreateWidget` "/Game/_Game/UI/WBP_Timer.WBP_Timer_C"))
  (set `self.TimerWidget` _returnvalue_2)
  (`UserWidget.AddToViewport` _returnvalue_2 0)
  (bind _output_get (set `self.CountdownTime` 10))
  (`/Game/_Game/UI/WBP_Timer.UpdateTimerText` _returnvalue_2 _output_get)
  (bind _returnvalue_3 (`KismetSystemLibrary.K2_SetTimerDelegate` (delegate `OnTimerTick`) 1.0 true))
  (set `self.TimerHandle` _returnvalue_3))

(event `RevealCorrectAnswer`
  (bind _returnvalue (`GameplayStatics.GetPlayerController` 0))
  ;[0.8796 0.8796 0.8796 0.502] REVEAL & ELIMINATION PHASE
  (set `self.bCanSelectAnswer` false)
  (set `PlayerController.bShowMouseCursor` false _returnvalue)
  (set `PlayerController.bEnableClickEvents` false _returnvalue)
  (`KismetArrayLibrary.Array_Clear` (`self.WrongPlatforms`))
  (bind _returnvalue_2 (`|GetDataTableRow` "/Game/_Game/Data/DT_QuestionBank.DT_QuestionBank" (`self.Current Question Row Name`))
    (:`then`
      (for _index (range 4)
        (if (!= _index (`.CorrectAnswerIndex_7_ED81544844DDBFA93D720D822A3BE6AC` (break `/Game/_Game/Data/S_Quiz` _returnvalue_2)))
          (bind _outactors (`GameplayStatics.GetAllActorsWithTag` (`KismetStringLibrary.Conv_StringToName` (`KismetStringLibrary.Concat_StrStr` "AnswerPlatform_" (`KismetStringLibrary.Conv_IntToString` _index)))))
          (bind _asbp_answer_platform (cast `/Game/_Game/BlueprintsGameplay/BP_AnswerPlatform` (`|GetArrayItem` _outactors)))
          (`KismetArrayLibrary.Array_Add` (`self.WrongPlatforms`) _asbp_answer_platform)))
      (`/Game/_Game/BlueprintsGameplay/BP_AnswerPlatform.EliminatePlatform` (`|GetArrayItem` (`self.WrongPlatforms`) (`self.RandomIndex`)))
      (set `self.RandomIndex` (`KismetMathLibrary.RandomIntegerInRange` 0 (- (`KismetArrayLibrary.Array_Length` (`self.WrongPlatforms`)) 1)))
      (`KismetArrayLibrary.Array_Remove` (`self.WrongPlatforms`) (`self.RandomIndex`))
      (`KismetSystemLibrary.Delay` 3.0)
      (for _array_element (`self.WrongPlatforms`)
        (`/Game/_Game/BlueprintsGameplay/BP_AnswerPlatform.EliminatePlatform` _array_element))
      (`self.FocusWinningPlatform`))))

(event `OnTimerTick`
  ;[0.8796 0.8796 0.8796 0.502] QUESTION & ANSWERING PHASE
  (bind _output_get (set `self.CountdownTime` (- (`self.CountdownTime`) 1)))
  (`/Game/_Game/UI/WBP_Timer.UpdateTimerText` (`self.TimerWidget`) _output_get)
  (if (<= _output_get 0)
    (`KismetSystemLibrary.K2_ClearAndInvalidateTimerHandle` (`self.TimerHandle`))))

(event `OnVotingTimeExpired`
  (bind _indexofmaxvalue (`KismetMathLibrary.MaxOfIntArray` (`self.DoorVotes`)))
  ;[0.8796 0.8796 0.8796 0.502] DOOR VOTING PHASE
  (`KismetSystemLibrary.PrintString` (`KismetStringLibrary.Conv_IntToString` _indexofmaxvalue))
  (`KismetArrayLibrary.Array_Clear` (`self.MatchingRowNames`))
  (bind _outrownames (`DataTableFunctionLibrary.GetDataTableRowNames` "/Game/_Game/Data/DT_QuestionBank.DT_QuestionBank"))
  (for _array_element _outrownames
    (bind _returnvalue (`|GetDataTableRow` "/Game/_Game/Data/DT_QuestionBank.DT_QuestionBank" _array_element)
      (:`then`
        (if (== (break `/Game/_Game/Data/S_Quiz` _returnvalue) (`|GetArrayItem` (`self.AvailableMainCategories`) _indexofmaxvalue))
          (`KismetArrayLibrary.Array_Add` (`self.MatchingRowNames`) _array_element)))))
  (`self.StartQuestionPhase`))

(event `SetupAnswerPlatforms`
  ;[0.8796 0.8796 0.8796 0.502] QUESTION & ANSWERING PHASE
  (`self.ResetAllPlatforms`)
  (`self.ResetAllPlayerTokens`)
  (bind _returnvalue (`|GetDataTableRow` "/Game/_Game/Data/DT_QuestionBank.DT_QuestionBank" (`self.Current Question Row Name`))
    (:`then`
      (for (_array_element _array_index) (`.Answers_15_5C8040D3432354FA3D5475B388D86669` (break `/Game/_Game/Data/S_Quiz` _returnvalue))
        (bind _outactors (`GameplayStatics.GetAllActorsWithTag` (`KismetStringLibrary.Conv_StringToName` (`KismetStringLibrary.Concat_StrStr` "AnswerPlatform_" (`KismetStringLibrary.Conv_IntToString` _array_index)))))
        (bind _asbp_answer_platform (cast `/Game/_Game/BlueprintsGameplay/BP_AnswerPlatform` (`|GetArrayItem` _outactors)))
        (`/Game/_Game/BlueprintsGameplay/BP_AnswerPlatform.UpdateAnswerText` _asbp_answer_platform _array_element)
        (`KismetSystemLibrary.Delay` 10.0)
        (`self.RevealCorrectAnswer`)))))

(event `StartDoorVoting`
  ;[0.8796 0.8796 0.8796 0.502] DOOR VOTING PHASE
  (`self.SetupDoorCategories`)
  (bind _outactors (`GameplayStatics.GetAllActorsWithTag` "DoorCamera"))
  (`PlayerController.SetViewTargetWithBlend` (`GameplayStatics.GetPlayerController` 0) (`|GetArrayItem` _outactors) 0.0 "VTBlend_Linear" 0.0 false))

(event `FocusWinningPlatform`
  ;[0.8796 0.8796 0.8796 0.502] REVEAL & ELIMINATION PHASE
  (bind _returnvalue (`|GetDataTableRow` "/Game/_Game/Data/DT_QuestionBank.DT_QuestionBank" "NewRow")
    (:`then`
      (`KismetSystemLibrary.Delay` 1.0)
      (bind _outactors (`GameplayStatics.GetAllActorsWithTag` (`KismetStringLibrary.Conv_StringToName` (`KismetStringLibrary.Concat_StrStr` "AnswerPlatform_" (`KismetStringLibrary.Conv_IntToString` (`.CorrectAnswerIndex_7_ED81544844DDBFA93D720D822A3BE6AC` (break `/Game/_Game/Data/S_Quiz` _returnvalue)))))))
      (bind _outactors_2 (`GameplayStatics.GetAllActorsWithTag` "AnswerCamera"))
      (bind (_direction _alpha) (`Timeline|Timeline` :!via `PlayFromStart`)
        (:`Update`
          (bind _output (`|GetArrayItem` _outactors_2))
          (`self.K2_SetActorRotation` _output (`KismetMathLibrary.RLerp` (`self.K2_GetActorRotation` _output) (`KismetMathLibrary.FindLookAtRotation` (`self.K2_GetActorLocation` _output) (`self.K2_GetActorLocation` (`|GetArrayItem` _outactors)))) false)
          (`CameraComponent.SetFieldOfView` (`self.GetComponentByClass` _output "/Script/Engine.CameraComponent") (`KismetMathLibrary.Lerp` 90.0 45.0 _alpha))
          (`KismetSystemLibrary.Delay` 5.0)
          (`self.OnQuestionEnded`))))))

(event `ResetAllPlatforms`
  ;[0.8796 0.8796 0.8796 0.502] QUESTION & ANSWERING PHASE
  (bind _outactors (`GameplayStatics.GetAllActorsOfClass` "/Game/_Game/BlueprintsGameplay/BP_AnswerPlatform.BP_AnswerPlatform_C"))
  (for _array_element _outactors
    (`/Game/_Game/BlueprintsGameplay/BP_AnswerPlatform.ResetPlatform` _array_element)))

(event `CastVote`
  (params (CategoryIndex :type Integer))
  (bind _votecounts (`self.VoteCounts`))
  ;[0.8796 0.8796 0.8796 0.502] DOOR VOTING PHASE
  (`KismetArrayLibrary.Array_Set` (`self.DoorVotes`) CategoryIndex (+ (`|GetArrayItem` (`self.DoorVotes`) CategoryIndex) 1))
  (`KismetArrayLibrary.Array_Set` _votecounts CategoryIndex (+ (`|GetArrayItem` _votecounts CategoryIndex) 1))
  (bind _outactors (`GameplayStatics.GetAllActorsWithTag` (`KismetStringLibrary.Conv_StringToName` (`KismetStringLibrary.Concat_StrStr` "Door" (`KismetStringLibrary.Conv_IntToString` CategoryIndex)))))
  (bind _aswbp_door_sign (cast `/Game/_Game/UI/WBP_DoorSign` (`WidgetComponent.GetUserWidgetObject` (`self.GetComponentByClass` (`|GetArrayItem` _outactors) "/Script/UMG.WidgetComponent"))))
  (`/Game/_Game/UI/WBP_DoorSign.AddVoteBadge` _aswbp_door_sign "/Engine/MapTemplates/TestCard.TestCard"))

(event `ResetAllDoors`
  ;[0.8796 0.8796 0.8796 0.502] DOOR VOTING PHASE
  (bind _outactors (`GameplayStatics.GetAllActorsOfClass` "/Game/_Game/BlueprintsGameplay/BP_Door.BP_Door_C"))
  (for _array_element _outactors
    (`/Game/_Game/BlueprintsGameplay/BP_Door.ResetDoor` _array_element)))

(fn `UserConstructionScript`)