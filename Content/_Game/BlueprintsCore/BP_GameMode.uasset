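; Game mode for a quiz party game, running question intro, category door voting, question, answering and reveal phases.
; One countdown timer advances phases by name as cameras switch between tagged views.
; Door votes, or a decelerating random shuffle without votes, filter DT_QuestionBank by category; wrong answer platforms drop and correct picks score.
; A separate stage/round flow, not called from BeginPlay, adds random augments and print-only mini-game and showdown stubs.
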(event `StartMiniGame`
  (`KismetSystemLibrary.PrintString` "\"Mini-Game Event Triggered!\"" true true (struct :`G` 0.615625 :`B` 0.072627 :`A` 1.0) 10.0))

(event `StartShowdown`
  (`KismetSystemLibrary.PrintString` "\"Final Stage Showdown Triggered!\"" true true (struct :`R` 0.615625 :`G` 0.013608 :`A` 1.0) 10.0))

(event `StartNextRound`
  (if (== (`self.RoundInStage`) 4)
    (if (>= (`self.CurrentStage`) (`self.MaxStages`))
      (`self.StartShowdown`)
      (else
        (`self.StartMiniGame`)))
    (elif (== (`self.RoundInStage`) (`self.StageAugmentRound`))
      (set `self.bIsAugmentActive` true)
      (bind _outrownames (`DataTableFunctionLibrary.GetDataTableRowNames` "/Game/_Game/Data/DT_Augments.DT_Augments"))
      (bind _returnvalue (`|GetDataTableRow` "/Game/_Game/Data/DT_Augments.DT_Augments" (`KismetArrayLibrary.Array_Random` _outrownames))
        (:`then`
          (set `self.ActiveAugmentData` _returnvalue)
          (bind _returnvalue_2 (`|CreateWidget` "/Game/_Game/UI/WBP_AugmentAlert.WBP_AugmentAlert_C"))
          (`/Game/_Game/UI/WBP_AugmentAlert.SetupAugmentDisplay` :`self` _returnvalue_2)
          (`UserWidget.AddToViewport` _returnvalue_2 0)
          (`self.StartPhaseTimer` 10 "AugmentSelection")
          (`self.StartDoorVoting`)))
      (else
        (set `self.bIsAugmentActive` false)
        (`self.StartDoorVoting`)))))

(event `StartNewStage`
  (set `self.RoundInStage` 1)
  (set `self.SelectedMainCategory` "")
  (`KismetArrayLibrary.Array_Clear` (`self.StageSubCategories`))
  (set `self.bIsAugmentActive` false)
  (set `self.StageAugmentRound` (`KismetMathLibrary.RandomIntegerInRange` 1 3))
  (`self.StartNextRound`))

(event `StartPhaseTimer`
  (params (Duration :type Integer) (TimerPhase :type Name))
  (`/Engine/EditorBlueprintResources/StandardMacros.IsValid` (`self.TimerWidget`)
    (:`Is Valid`
      _)
    (:`Is Not Valid`
      (bind _returnvalue (`|CreateWidget` "/Game/_Game/UI/WBP_Timer.WBP_Timer_C"))
      (bind _output_get (set `self.TimerWidget` _returnvalue))))
  (`Widget.SetVisibility` _output_get "Visible")
  (if (not (`Widget.IsInViewport` _output_get))
    (`UserWidget.AddToViewport` _output_get 10))
  (set `self.ActiveTimerPhase` TimerPhase)
  (bind _output_get_2 (set `self.CountdownTime` Duration))
  (`/Game/_Game/UI/WBP_Timer.UpdateTimerText` (`self.TimerWidget`) _output_get_2)
  (bind _returnvalue_2 (`KismetSystemLibrary.K2_SetTimerDelegate` (delegate `OnTimerTick`) 1.0 true))
  (set `self.TimerHandle` _returnvalue_2))

(event `OnTimerTick`
  (bind _output_get (set `self.CountdownTime` (- (`self.CountdownTime`) 1)))
  (`/Game/_Game/UI/WBP_Timer.UpdateTimerText` (`self.TimerWidget`) _output_get)
  (if (<= _output_get 0)
    (`KismetSystemLibrary.K2_ClearAndInvalidateTimerHandle` (`self.TimerHandle`))
    (switch `name` (`self.ActiveTimerPhase`)
      (:`Voting`
        (`self.OnVotingTimeExpired`))
      (:`Question`
        (`Widget.RemoveFromParent` (`self.QuestionShowcase`))
        (`self.StartAnsweringPhase`))
      (:`Answering`
        (`self.RevealCorrectAnswer`)
        (`self.AwardSurvivingPlayers`))
      (:`QuestionIntro`
        (`Widget.RemoveFromParent` (`self.QuestionIntro`))
        (`self.StartDoorVoting`)))))

(event `self.ReceiveBeginPlay`
  (bind _returnvalue (`|CreateWidget` "/Game/_Game/UI/WBP_Timer.WBP_Timer_C"))
  (bind _output_get (set `self.TimerWidget` _returnvalue))
  (`UserWidget.AddToViewport` _returnvalue 10)
  (`UserWidget.AddToViewport` _output_get 10)
  (`self.SetupPlayerCards`)
  (`self.SetupMatchEvents`)
  (`self.StartNextQuestion`))

(event `AddScore`
  (params (`Player Index` :type Integer) (`Point to Add` :type Integer))
  (`KismetArrayLibrary.Array_Set` (`self.PlayerScores`) `Player Index` (+ (`|GetArrayItem` (`self.PlayerScores`) `Player Index`) `Point to Add`) true)
  (`KismetSystemLibrary.PrintString` "score ")
  (`/Game/_Game/UI/WBP_PlayerCard.UpdateCardUI` (`|GetArrayItem` (`self.PlayerCardWidgets`) `Player Index`) `Player Index`))

(event `StartDoorShuffle`
  (bind _outactors (`GameplayStatics.GetAllActorsOfClass` "/Game/_Game/BlueprintsGameplay/BP_Door.BP_Door_C"))
  (set `self.AllDoors` _outactors)
  (set `self.ShuffleDelay` 0.05)
  (set `self.RemainingHops` (+ (`self.ChosenDoorIndex`) 16))
  (`self.RunShuffleStep`))

(event `ResetAllPlayerTokens`
  (bind _outactors (`GameplayStatics.GetAllActorsOfClass` "/Game/_Game/BlueprintsCore/BP_PlayerToken.BP_PlayerToken_C"))
  (for _array_element _outactors
    (`self.K2_DestroyActor` _array_element))
  (for _index (range (`self.TotalPlayers`))
    (`KismetArrayLibrary.Array_Set` (`self.PlayerChoices`) _index -1)))

(event `SetupPlayerCards`
  (for _index (range (`self.TotalPlayers`))
    (bind _returnvalue (`|CreateWidget` "/Game/_Game/UI/WBP_PlayerCard.WBP_PlayerCard_C" null null))
    (`KismetArrayLibrary.Array_Add` (`self.PlayerCardWidgets`) _returnvalue)
    (`UserWidget.AddToViewport` _returnvalue 0)
    (`UserWidget.SetPositionInViewport` _returnvalue (`KismetMathLibrary.MakeVector2D` (`KismetMathLibrary.Conv_IntToDouble` (* _index 300)) 50.0) true)
    (`KismetArrayLibrary.Array_Add` (`self.PlayerScores`))))

(event `RegisterPlayerChoice`
  (params (PlayerIndex :type Integer) (ChosenPlatformIndex :type Integer))
  (`KismetArrayLibrary.Array_Set` (`self.PlayerChoices`) PlayerIndex ChosenPlatformIndex))

(event `RunShuffleStep`
  (for _array_element (`self.AllDoors`)
    (`/Game/_Game/BlueprintsGameplay/BP_Door.SetDoorHighlight` _array_element false))
  (`/Game/_Game/BlueprintsGameplay/BP_Door.SetDoorHighlight` (`|GetArrayItem` (`self.AllDoors`) (`self.CurrentShuffleIndex`)) true)
  (set `self.CurrentShuffleIndex` (mod (+ (`self.CurrentShuffleIndex`) 1) (`KismetArrayLibrary.Array_Length` (`self.AllDoors`))))
  (bind _output_get (set `self.RemainingHops` (- (`self.RemainingHops`) 1)))
  (if (<= _output_get 0)
    (`KismetSystemLibrary.Delay` 1.0)
    (`KismetSystemLibrary.PrintString` "Shuffle Finished")
    (`KismetArrayLibrary.Array_Clear` (`self.MatchingRowNames`))
    (bind _outrownames (`DataTableFunctionLibrary.GetDataTableRowNames` "/Game/_Game/Data/DT_QuestionBank.DT_QuestionBank"))
    (for _array_element_2 _outrownames
      (bind _returnvalue (`|GetDataTableRow` "/Game/_Game/Data/DT_QuestionBank.DT_QuestionBank" _array_element_2)
        (:`then`
          (if (== (break `/Game/_Game/Data/S_Quiz` _returnvalue) (`|GetArrayItem` (`self.AvailableMainCategories`) (`self.ChosenDoorIndex`)))
            (`KismetArrayLibrary.Array_Add` (`self.MatchingRowNames`) _array_element_2)
            (`KismetSystemLibrary.PrintString` (`KismetStringLibrary.Conv_NameToString` _array_element_2))))))
    (`KismetSystemLibrary.PrintString` "complete" true true (struct :`G` 0.66 :`B` 1.0 :`A` 1.0) 10.0)
    (`self.StartQuestionPhase`)
    (else
      (bind _output_get_2 (set `self.ShuffleDelay` (+ (`self.ShuffleDelay`) 0.025)))
      (`KismetSystemLibrary.Delay` _output_get_2)
      (`self.RunShuffleStep`))))

(event `AwardSurvivingPlayers`
  ;[0.8796 0.8796 0.8796 0.502] QUESTION & ANSWERING PHASE
  (`/Engine/EditorBlueprintResources/StandardMacros.DoOnce` false :!label _label
    (:`Completed`
      (for _index (range (`self.TotalPlayers`))
        (if (== (`self.CorrectAnswerIndex`) (`|GetArrayItem` (`self.PlayerChoices`) _index))
          (`self.AddScore` _index 100))))))

(event `ResetScoreGate`
  ;[0.8796 0.8796 0.8796 0.502] QUESTION & ANSWERING PHASE
  (goto _label :!via `Reset`))

(event `OnQuestionEnded`
  ;[0.8796 0.8796 0.8796 0.502] GAME LOOP & PROGRESSION
  (`KismetSystemLibrary.K2_ClearAndInvalidateTimerHandle` (`self.TimerHandle`))
  (`Widget.RemoveFromParent` (`self.TimerWidget`))
  (`self.ResetAllDoors`)
  (if (== (mod (`self.CurrentQuestionNumber`) 3) 0)
    (`KismetSystemLibrary.PrintString` "EVENT TIME! Triggering event...")
    (`self.StartDoorVoting`)
    (else
      (set `self.CurrentQuestionNumber` (+ (`self.CurrentQuestionNumber`) 1))
      (`self.StartNextQuestion`))))

(event `SetupDoorCategories`
  ;[0.8796 0.8796 0.8796 0.502] DOOR VOTING PHASE
  (bind _outrownames (`DataTableFunctionLibrary.GetDataTableRowNames` "/Game/_Game/Data/DT_QuestionBank.DT_QuestionBank"))
  (for _array_element _outrownames
    (bind _returnvalue (`|GetDataTableRow` "/Game/_Game/Data/DT_QuestionBank.DT_QuestionBank" _array_element)
      (:`then`
        (`KismetArrayLibrary.Array_AddUnique` (`self.AvailableMainCategories`) (`KismetStringLibrary.Conv_NameToString` (break `/Game/_Game/Data/S_Quiz` _returnvalue))))))
  (`KismetArrayLibrary.Array_Shuffle` (`self.AvailableMainCategories`))
  (for _index (range 4)
    (bind _outactors (`GameplayStatics.GetAllActorsWithTag` (`KismetStringLibrary.Conv_StringToName` (`KismetStringLibrary.Concat_StrStr` "Door" (`KismetStringLibrary.Conv_IntToString` _index)))))
    (bind _asbp_door (cast `/Game/_Game/BlueprintsGameplay/BP_Door` (`|GetArrayItem` _outactors)))
    (`/Game/_Game/BlueprintsGameplay/BP_Door.SetDoorCategory` _asbp_door (`|GetArrayItem` (`self.AvailableMainCategories`) _index)))
  (set `PlayerController.bShowMouseCursor` true (`GameplayStatics.GetPlayerController` 0))
  (set `PlayerController.bEnableClickEvents` true (`GameplayStatics.GetPlayerController` 0))
  ;;[0 1 0 0.5] Phase Timer
  (`self.StartPhaseTimer` 10 "Voting"))

(event `StartNextQuestion`
  ;[0.8796 0.8796 0.8796 0.502] QUESTION & ANSWERING PHASE
  (bind _returnvalue (`|CreateWidget` "/Game/_Game/UI/WBP_QuestionIntro.WBP_QuestionIntro_C"))
  (`/Game/_Game/UI/WBP_QuestionIntro.fn_SetBannerText` _returnvalue (`self.CurrentQuestionNumber`) "Knowledge Party")
  (set `self.QuestionIntro` _returnvalue)
  (`UserWidget.AddToViewport` _returnvalue 0)
  ;;[0 1 0 0.5] Phase Timer
  (`self.StartPhaseTimer` 7 "QuestionIntro")
  (`self.ResetScoreGate`))

(event `SetupMatchEvents`
  (bind _activeeventslist (`self.ActiveEventsList`))
  ;[0.8796 0.8796 0.8796 0.502] Comment
  (`KismetArrayLibrary.Array_Shuffle` (`self.AvailableEvents`))
  (`KismetArrayLibrary.Array_Clear` _activeeventslist)
  (`KismetArrayLibrary.Array_Add` _activeeventslist (`|GetArrayItem` (`self.AvailableEvents`)))
  (`KismetArrayLibrary.Array_Add` _activeeventslist (`|GetArrayItem` (`self.AvailableEvents`) 1))
  (`KismetArrayLibrary.Array_Add` _activeeventslist "NewEnumerator3"))

(event `StartQuestionPhase`
  ;[0.8796 0.8796 0.8796 0.502] QUESTION & ANSWERING PHASE
  (if (> (`KismetArrayLibrary.Array_Length` (`self.MatchingRowNames`)) 0)
    (bind _output_get (set `self.Current Question Row Name` (`KismetArrayLibrary.Array_Random` (`self.MatchingRowNames`))))
    (bind _returnvalue (`|GetDataTableRow` "/Game/_Game/Data/DT_QuestionBank.DT_QuestionBank" _output_get)
      (:`then`
        (bind _outactors (`GameplayStatics.GetAllActorsWithTag` "QuestionCamera"))
        (`PlayerController.SetViewTargetWithBlend` (`GameplayStatics.GetPlayerController` 0) (`|GetArrayItem` _outactors) 1.5 "VTBlend_EaseInOut" 0.0 false)
        (bind _returnvalue_2 (`|CreateWidget` "/Game/_Game/UI/WBP_QuestionShowcase.WBP_QuestionShowcase_C" null (`.QuestionText_2_3D36EEE940F58E65A419A48BB2DB8745` (break `/Game/_Game/Data/S_Quiz` _returnvalue))))
        (set `self.QuestionShowcase` _returnvalue_2)
        (`UserWidget.AddToViewport` _returnvalue_2 0)
        ;;[0 1 0 0.5] Phase Timer
        (`self.StartPhaseTimer` 10 "Question"))
      (:`RowNotFound`
        (`KismetSystemLibrary.PrintString` "ERROR: Question row missing from DT_QuestionBank!" true true (struct :`R` 0.665625 :`G` 0.018749 :`A` 1.0) 20.0)))
    (else
      (`KismetSystemLibrary.PrintString` "ERROR: No matching questions found for selected category!" true true (struct :`R` 1.0 :`G` 0.007416 :`A` 1.0) 20.0))))

(event `OnVotingTimeFinished`)

(event `StartAnsweringPhase`
  (bind _returnvalue (`GameplayStatics.GetPlayerController` 0))
  ;[0.8796 0.8796 0.8796 0.502] QUESTION & ANSWERING PHASE
  (bind _outactors (`GameplayStatics.GetAllActorsWithTag` "AnswerCamera"))
  (`PlayerController.SetViewTargetWithBlend` (`GameplayStatics.GetPlayerController` 0) (`|GetArrayItem` _outactors) 1.0 "VTBlend_EaseInOut" 0.0 false)
  (`self.SetupAnswerPlatforms`)
  (set `self.bCanSelectAnswer` true)
  (set `PlayerController.bShowMouseCursor` true _returnvalue)
  (set `PlayerController.bEnableClickEvents` true _returnvalue))

(event `RevealCorrectAnswer`
  (bind _returnvalue (`GameplayStatics.GetPlayerController` 0))
  ;[0.8796 0.8796 0.8796 0.502] REVEAL & ELIMINATION PHASE
  (set `self.bCanSelectAnswer` false)
  (set `PlayerController.bShowMouseCursor` false _returnvalue)
  (set `PlayerController.bEnableClickEvents` false _returnvalue)
  (`KismetArrayLibrary.Array_Clear` (`self.WrongPlatforms`))
  (bind _returnvalue_2 (`|GetDataTableRow` "/Game/_Game/Data/DT_QuestionBank.DT_QuestionBank" (`self.Current Question Row Name`))
    (:`then`
      (set `self.CorrectAnswerIndex` (`.CorrectAnswerIndex_7_ED81544844DDBFA93D720D822A3BE6AC` (break `/Game/_Game/Data/S_Quiz` _returnvalue_2)))
      (for _index (range 4)
        (if (!= _index (`.CorrectAnswerIndex_7_ED81544844DDBFA93D720D822A3BE6AC` (break `/Game/_Game/Data/S_Quiz` _returnvalue_2)))
          (bind _outactors (`GameplayStatics.GetAllActorsWithTag` (`KismetStringLibrary.Conv_StringToName` (`KismetStringLibrary.Concat_StrStr` "AnswerPlatform_" (`KismetStringLibrary.Conv_IntToString` _index)))))
          (bind _asbp_answer_platform (cast `/Game/_Game/BlueprintsGameplay/BP_AnswerPlatform` (`|GetArrayItem` _outactors)))
          (`KismetArrayLibrary.Array_Add` (`self.WrongPlatforms`) _asbp_answer_platform)))
      (set `self.RandomIndex` (`KismetMathLibrary.RandomIntegerInRange` 0 (- (`KismetArrayLibrary.Array_Length` (`self.WrongPlatforms`)) 1)))
      (`/Game/_Game/BlueprintsGameplay/BP_AnswerPlatform.EliminatePlatform` (`|GetArrayItem` (`self.WrongPlatforms`) (`self.RandomIndex`)))
      (`KismetArrayLibrary.Array_Remove` (`self.WrongPlatforms`) (`self.RandomIndex`))
      (`KismetSystemLibrary.Delay` 3.0)
      (for _array_element (`self.WrongPlatforms`)
        (`/Game/_Game/BlueprintsGameplay/BP_AnswerPlatform.EliminatePlatform` _array_element))
      (`self.FocusWinningPlatform`)
      (`KismetSystemLibrary.Delay` 1.5)
      (`self.AwardSurvivingPlayers`))))

(event `OnVotingTimeExpired`
  (bind (_indexofmaxvalue _maxvalue) (`KismetMathLibrary.MaxOfIntArray` (`self.DoorVotes`)))
  ;[0.8796 0.8796 0.8796 0.502] DOOR VOTING PHASE
  (`KismetSystemLibrary.PrintString` (`KismetStringLibrary.Conv_IntToString` _indexofmaxvalue))
  (if (> _maxvalue 0)
    (set `self.ChosenDoorIndex` _indexofmaxvalue)
    (`KismetArrayLibrary.Array_Clear` (`self.MatchingRowNames`))
    (bind _outrownames (`DataTableFunctionLibrary.GetDataTableRowNames` "/Game/_Game/Data/DT_QuestionBank.DT_QuestionBank"))
    (for _array_element _outrownames
      (bind _returnvalue (`|GetDataTableRow` "/Game/_Game/Data/DT_QuestionBank.DT_QuestionBank" _array_element)
        (:`then`
          (if (== (break `/Game/_Game/Data/S_Quiz` _returnvalue) (`|GetArrayItem` (`self.AvailableMainCategories`) (`self.ChosenDoorIndex`)))
            (`KismetArrayLibrary.Array_Add` (`self.MatchingRowNames`) _array_element)))))
    (`self.StartQuestionPhase`)
    (else
      (set `self.ChosenDoorIndex` (`KismetMathLibrary.RandomIntegerInRange` 0 3))
      (`self.StartDoorShuffle`)
      (`KismetSystemLibrary.PrintString` "falseeeeeee" true true (struct :`G` 0.66 :`B` 1.0 :`A` 1.0) 7.0))))

(event `SetupAnswerPlatforms`
  ;[0.8796 0.8796 0.8796 0.502] QUESTION & ANSWERING PHASE
  (`self.ResetAllPlatforms`)
  (`self.ResetAllPlayerTokens`)
  (bind _returnvalue (`|GetDataTableRow` "/Game/_Game/Data/DT_QuestionBank.DT_QuestionBank" (`self.Current Question Row Name`))
    (:`then`
      (for (_array_element _array_index) (`.Answers_15_5C8040D3432354FA3D5475B388D86669` (break `/Game/_Game/Data/S_Quiz` _returnvalue))
        (bind _outactors (`GameplayStatics.GetAllActorsWithTag` (`KismetStringLibrary.Conv_StringToName` (`KismetStringLibrary.Concat_StrStr` "AnswerPlatform_" (`KismetStringLibrary.Conv_IntToString` _array_index)))))
        (bind _asbp_answer_platform (cast `/Game/_Game/BlueprintsGameplay/BP_AnswerPlatform` (`|GetArrayItem` _outactors)))
        (`/Game/_Game/BlueprintsGameplay/BP_AnswerPlatform.UpdateAnswerText` _asbp_answer_platform _array_element)
        ;;[0 1 0 0.5] Phase Timer
        (`self.StartPhaseTimer` 15 "Answering")))))

(event `StartDoorVoting`
  ;[0.8796 0.8796 0.8796 0.502] DOOR VOTING PHASE
  (`self.SetupDoorCategories`)
  (bind _outactors (`GameplayStatics.GetAllActorsWithTag` "DoorCamera"))
  (`PlayerController.SetViewTargetWithBlend` (`GameplayStatics.GetPlayerController` 0) (`|GetArrayItem` _outactors) 0.0 "VTBlend_Linear" 0.0 false))

(event `FocusWinningPlatform`
  ;[0.8796 0.8796 0.8796 0.502] REVEAL & ELIMINATION PHASE
  (bind _returnvalue (`|GetDataTableRow` "/Game/_Game/Data/DT_QuestionBank.DT_QuestionBank" "NewRow")
    (:`then`
      (`KismetSystemLibrary.Delay` 1.0)
      (bind _outactors (`GameplayStatics.GetAllActorsWithTag` (`KismetStringLibrary.Conv_StringToName` (`KismetStringLibrary.Concat_StrStr` "AnswerPlatform_" (`KismetStringLibrary.Conv_IntToString` (`.CorrectAnswerIndex_7_ED81544844DDBFA93D720D822A3BE6AC` (break `/Game/_Game/Data/S_Quiz` _returnvalue)))))))
      (bind _outactors_2 (`GameplayStatics.GetAllActorsWithTag` "AnswerCamera"))
      (bind (_direction _alpha) (`Timeline|Timeline` :!via `PlayFromStart`)
        (:`Update`
          (bind _output (`|GetArrayItem` _outactors_2))
          (`self.K2_SetActorRotation` _output (`KismetMathLibrary.RLerp` (`self.K2_GetActorRotation` _output) (`KismetMathLibrary.FindLookAtRotation` (`self.K2_GetActorLocation` _output) (`self.K2_GetActorLocation` (`|GetArrayItem` _outactors)))) false)
          (`CameraComponent.SetFieldOfView` (`self.GetComponentByClass` _output "/Script/Engine.CameraComponent") (`KismetMathLibrary.Lerp` 90.0 45.0 _alpha))
          (`KismetSystemLibrary.Delay` 5.0)
          (`self.OnQuestionEnded`))))))

(event `ResetAllPlatforms`
  ;[0.8796 0.8796 0.8796 0.502] QUESTION & ANSWERING PHASE
  (bind _outactors (`GameplayStatics.GetAllActorsOfClass` "/Game/_Game/BlueprintsGameplay/BP_AnswerPlatform.BP_AnswerPlatform_C"))
  (for _array_element _outactors
    (`/Game/_Game/BlueprintsGameplay/BP_AnswerPlatform.ResetPlatform` _array_element)))

(event `CastVote`
  (params (CategoryIndex :type Integer))
  (bind _votecounts (`self.VoteCounts`))
  ;[0.8796 0.8796 0.8796 0.502] DOOR VOTING PHASE
  (`KismetArrayLibrary.Array_Set` (`self.DoorVotes`) CategoryIndex (+ (`|GetArrayItem` (`self.DoorVotes`) CategoryIndex) 1))
  (`KismetArrayLibrary.Array_Set` _votecounts CategoryIndex (+ (`|GetArrayItem` _votecounts CategoryIndex) 1))
  (bind _outactors (`GameplayStatics.GetAllActorsWithTag` (`KismetStringLibrary.Conv_StringToName` (`KismetStringLibrary.Concat_StrStr` "Door" (`KismetStringLibrary.Conv_IntToString` CategoryIndex)))))
  (bind _aswbp_door_sign (cast `/Game/_Game/UI/WBP_DoorSign` (`WidgetComponent.GetUserWidgetObject` (`self.GetComponentByClass` (`|GetArrayItem` _outactors) "/Script/UMG.WidgetComponent"))))
  (`/Game/_Game/UI/WBP_DoorSign.AddVoteBadge` _aswbp_door_sign "/Engine/MapTemplates/TestCard.TestCard"))

(event `ResetAllDoors`
  ;[0.8796 0.8796 0.8796 0.502] DOOR VOTING PHASE
  (bind _outactors (`GameplayStatics.GetAllActorsOfClass` "/Game/_Game/BlueprintsGameplay/BP_Door.BP_Door_C"))
  (for _array_element _outactors
    (`/Game/_Game/BlueprintsGameplay/BP_Door.ResetDoor` _array_element)))

(fn `GetPlayersSortedByScore`
  (returns (SortedPlayers :type "Array of /Game/_Game/BlueprintsCore/BP_PlayerToken Object Reference"))
  (locals (UnsortedPlayers :type "Array of /Game/_Game/BlueprintsCore/BP_PlayerToken Object Reference") (SortedResult :type "Array of /Game/_Game/BlueprintsCore/BP_PlayerToken Object Reference") (LowestPlayer :type "/Game/_Game/BlueprintsCore/BP_PlayerToken Object Reference") (LowestScore :type Integer))
  (bind _outactors (`GameplayStatics.GetAllActorsOfClass` "/Game/_Game/BlueprintsCore/BP_PlayerToken.BP_PlayerToken_C"))
  (bind _output_get (set `local.UnsortedPlayers` _outactors))
  (while (> (`KismetArrayLibrary.Array_Length` _output_get) 0)
    (bind _output_get_2 (set `local.LowestPlayer` (`|GetArrayItem` (`local.UnsortedPlayers`))))
    (bind _output_get_3 (set `local.LowestScore` (`/Game/_Game/BlueprintsCore/BP_PlayerToken.Score` _output_get_2)))
    (for _array_element (`local.UnsortedPlayers`)
      (bind _score (`/Game/_Game/BlueprintsCore/BP_PlayerToken.Score` _array_element))
      (if (< _score _output_get_3)
        (set `local.LowestPlayer` null)
        (set `local.LowestScore` _score)))
    (`KismetArrayLibrary.Array_Add` (`local.SortedResult`) (`local.LowestPlayer`))
    (`KismetArrayLibrary.Array_RemoveItem` (`local.UnsortedPlayers`) (`local.LowestPlayer`)))
  (return (`local.SortedResult`)))

(fn `GetStageTargetDifficulty`
  (returns (TargetDifficulty :type "/Game/_Game/Data/E_QuestionDifficulty Enum"))
  (switch `int` (`self.CurrentStage`)
    (:`Default`
      (return "NewEnumerator2"))
    (:`1`
      (return "NewEnumerator0"))
    (:`2`
      (return "NewEnumerator1"))))

(fn `UserConstructionScript`)