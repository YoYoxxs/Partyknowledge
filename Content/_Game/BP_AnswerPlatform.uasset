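; BP_AnswerPlatform is a clickable platform actor that displays an answer's text and receives a player token when selected.
; A mesh click casts the game mode to BP_GameState and, if CanSelectAnswer is true, spawns a BP_PlayerToken above TokenAnchor.
; A timeline then lerps the token down onto the anchor.
; Separate events update the displayed text and eliminate the platform by hiding it and disabling collision.
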(event `self.ReceiveBeginPlay`)

(event `UpdateAnswerText`
  (params (NewText :type Text))
  (`TextRenderComponent.K2_SetText` (`self.Txt_AnswerDisplay`) NewText))

(event `self.StaticMesh.OnClicked`
  (params (TouchedComponent :type "PrimitiveComponent Object Reference") (ButtonPressed :type "Key Structure"))
  (bind _asbp_game_state (cast `/Game/_Game/BP_GameState` (`GameplayStatics.GetGameMode`)))
  (if (`/Game/_Game/BP_GameState.bCanSelectAnswer` _asbp_game_state)
    (`self.DropToken`)))

(event `DropToken`
  (bind _returnvalue (`SceneComponent.K2_GetComponentLocation` (`self.TokenAnchor`)))
  (bind _returnvalue_2 (+ _returnvalue (0.0 0.0 500.0)))
  (bind _returnvalue_3 (`|SpawnActorFromClass` "/Game/_Game/BP_PlayerToken.BP_PlayerToken_C" (`KismetMathLibrary.MakeTransform` _returnvalue_2) "Undefined" "MultiplyWithRoot" null null))
  (bind _output_get (set `self.Spawned Token` _returnvalue_3))
  (bind (_direction _alpha) (`Timeline|TL_DropToken` :!via `PlayFromStart`)
    (:`Update`
      (`self.K2_SetActorLocation` _output_get (`KismetMathLibrary.VLerp` _returnvalue_2 _returnvalue _alpha) false false))))

(event `EliminatePlatform`
  (`self.SetActorHiddenInGame` true)
  (`self.SetActorEnableCollision` false))

(fn `UserConstructionScript`)