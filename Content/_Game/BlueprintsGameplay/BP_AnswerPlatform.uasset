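; Clickable answer platform that displays an answer text and can be eliminated or reset by toggling its visibility and collision.
; When the game mode allows selection, a click drops player 0's token and registers that platform as the choice.
; DropToken replaces that player's existing token, links the new one to its player card widget from the game mode, and lowers it onto TokenAnchor with a timeline lerp.
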(event `self.ReceiveBeginPlay`)

(event `UpdateAnswerText`
  (params (NewText :type Text))
  (`TextRenderComponent.K2_SetText` (`self.Txt_AnswerDisplay`) NewText))

(event `self.StaticMesh.OnClicked`
  (params (TouchedComponent :type "PrimitiveComponent Object Reference") (ButtonPressed :type "Key Structure"))
  (bind _asbp_game_mode (cast `/Game/_Game/BlueprintsCore/BP_GameMode` (`GameplayStatics.GetGameMode`)))
  (if (`/Game/_Game/BlueprintsCore/BP_GameMode.bCanSelectAnswer` _asbp_game_mode)
    (`self.DropToken` 0)
    (`/Game/_Game/BlueprintsCore/BP_GameMode.RegisterPlayerChoice` _asbp_game_mode 0 (`self.PlatformIndex`))))

(event `ResetPlatform`
  (`self.SetActorHiddenInGame` false)
  (`self.SetActorEnableCollision` true))

(event `DropToken`
  (params (PlayerIndex :type Integer))
  (bind _returnvalue (`SceneComponent.K2_GetComponentLocation` (`self.TokenAnchor`)))
  (bind _returnvalue_2 (+ _returnvalue (0.0 0.0 500.0)))
  ;[1 1 1 0.7] Comment
  (bind _outactors (`GameplayStatics.GetAllActorsOfClass` "/Game/_Game/BlueprintsCore/BP_PlayerToken.BP_PlayerToken_C"))
  (for _array_element _outactors
    (if (== (`/Game/_Game/BlueprintsCore/BP_PlayerToken.PlayerIndex` _array_element) PlayerIndex)
      (`self.K2_DestroyActor` _array_element)))
  (bind _returnvalue_3 (`|SpawnActorFromClass` "/Game/_Game/BlueprintsCore/BP_PlayerToken.BP_PlayerToken_C" (`KismetMathLibrary.MakeTransform` _returnvalue_2) "Undefined" "MultiplyWithRoot" null null))
  (bind _output_get (set `self.Spawned Token` _returnvalue_3))
  (set `/Game/_Game/BlueprintsCore/BP_PlayerToken.PlayerIndex` PlayerIndex _output_get)
  (bind _asbp_game_mode (cast `/Game/_Game/BlueprintsCore/BP_GameMode` (`GameplayStatics.GetGameMode`)))
  (bind _output (`|GetArrayItem` (`/Game/_Game/BlueprintsCore/BP_GameMode.PlayerCardWidgets` _asbp_game_mode) PlayerIndex))
  (set `/Game/_Game/BlueprintsCore/BP_PlayerToken.PlayerCard widget` _output _returnvalue_3)
  (set `/Game/_Game/UI/WBP_PlayerCard.OwningPlayerToken` _returnvalue_3 _output)
  (`/Game/_Game/UI/WBP_PlayerCard.UpdateCardUI` _output PlayerIndex)
  (bind (_direction _alpha) (`Timeline|TL_DropToken` :!via `PlayFromStart`)
    (:`Update`
      (`/Engine/EditorBlueprintResources/StandardMacros.IsValid` (`self.Spawned Token`)
        (:`Is Valid`
          (`self.K2_SetActorLocation` _output_get (`KismetMathLibrary.VLerp` _returnvalue_2 _returnvalue _alpha) false false))))))

(event `EliminatePlatform`
  (`self.SetActorHiddenInGame` true)
  (`self.SetActorEnableCollision` false))

(fn `UserConstructionScript`)